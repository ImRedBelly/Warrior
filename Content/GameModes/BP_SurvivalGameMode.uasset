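; Survival game mode Blueprint that presents wave progress to the player as on-screen announcements.
; On BeginPlay it binds to the game mode's state change event and switches on the new state.
; Two helper functions create text widgets, with countdowns for incoming and completed waves and without for the current wave number.
; The final wave also overrides the enemy spawn delay and adds a "Last Wave" message, while victory and player death only print debug strings.
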(event `self.ReceiveBeginPlay`
  (add `self.OnSurvivalGameModeStateChanged` (delegate `OnSurvivalGameModeStateChanged_Event`)))

(event `OnSurvivalGameModeStateChanged_Event` :!signature `self.OnSurvivalGameModeStateChanged`
  (params (CurrentState :type "EWarriorSurvivalGameModeState Enum" :default "WaitSpawnNewWave"))
  (switch `EWarriorSurvivalGameModeState` CurrentState
    (:`WaitSpawnNewWave`
      (`self.CreateWaveWidgetWithCountDown` "New Wave Coming In" (`self.SpawnNewWaveWaitTime`)))
    (:`SpawningNewWave`
      (`self.CreateWaveWidgetNoCountDown` (`|FormatText` "Wave {CurrentWaveCount}" (`self.CurrentWaveCount`)))
      (if (== (`self.CurrentWaveCount`) (`self.TotalWavesToSpawn`))
        (set `self.SpawnEnemiesDelayTime` 4.0)
        (`KismetSystemLibrary.Delay` 2.0)
        (`self.CreateWaveWidgetNoCountDown` "Last Wave")))
    (:`WaveCompleted`
      (`self.CreateWaveWidgetWithCountDown` (`|FormatText` "Wave {CurrentWaveCount} Completed" (`self.CurrentWaveCount`)) (`self.WaveCompletedWaitTime`)))
    (:`AllWavesDone`
      (`KismetSystemLibrary.PrintString` "AAAAAAAAA" true true (struct :`R` 0.397837 :`G` 1.0 :`B` 0.26565 :`A` 1.0) 8.0 "1"))
    (:`PlayerDied`
      (`KismetSystemLibrary.PrintString` "Здфнук Вшув" true true (struct :`R` 1.0 :`B` 0.214916 :`A` 1.0) 8.0 "1"))))

(fn `CreateWaveWidgetNoCountDown`
  (params (TextContentToDisplay :type Text))
  (bind _returnvalue (`|CreateWidget` "/Game/Widgets/GameModeWidgets/WBP_WaitTextNoCountDown.WBP_WaitTextNoCountDown_C"))
  (`UserWidget.AddToViewport` _returnvalue 0)
  (`TextBlock.SetText` (`/Game/Widgets/GameModeWidgets/WBP_WaitTextNoCountDown.TextBlock_WaveText` _returnvalue) (`local.TextContentToDisplay`)))

(fn `CreateWaveWidgetWithCountDown`
  (params (TextContentToDisplay :type Text) (InTotalCountDownTime :type "Float (double-precision)"))
  (bind _returnvalue (`|CreateWidget` "/Game/Widgets/GameModeWidgets/WBP_WaitTextWithCountDown.WBP_WaitTextWithCountDown_C"))
  (`UserWidget.AddToViewport` _returnvalue 0)
  (`TextBlock.SetText` (`/Game/Widgets/GameModeWidgets/WBP_WaitTextWithCountDown.TextBlock_WaveText` _returnvalue) (`local.TextContentToDisplay`))
  (`/Game/Widgets/GameModeWidgets/WBP_WaitTextWithCountDown.StartCounDown` _returnvalue (`local.InTotalCountDownTime`)))

(fn `UserConstructionScript`)