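; Base projectile Blueprint that handles sound and visual effects for spawn, flight and impact.
; On BeginPlay it plays a spawn sound, attaches a flight sound to the root and spawns a muzzle system facing the actor's forward vector.
; The OnSpawnHitFX event plays an impact sound and spawns an impact system at the supplied hit location.
; Each effect is skipped when its asset variable is not valid.
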(event `self.ReceiveBeginPlay`
  (`|ExecutionSequence`
    (:`then_0`
      (bind _spawnsound (`self.SpawnSound`)
        (:`then`
          (`GameplayStatics.PlaySoundAtLocation` _spawnsound (`self.K2_GetActorLocation`) (struct) 1.0 1.0 0.0 null null null null))
        (:`else`)))
    (:`then_1`
      (bind _flysound (`self.FlySound`)
        (:`then`
          (`GameplayStatics.SpawnSoundAttached` _flysound (`self.RootComponent`) "None" (0.0 0.0 0.0) (struct) "KeepRelativeOffset" true 1.0 1.0 0.0 null null))
        (:`else`)))
    (:`then_2`
      (bind _muzzlefx (`self.MuzzleFX`)
        (:`then`
          (`NiagaraFunctionLibrary.SpawnSystemAtLocation` _muzzlefx (`self.K2_GetActorLocation`) (`KismetMathLibrary.Conv_VectorToRotator` (`self.GetActorForwardVector`))))
        (:`else`)))))

(event `self.BP_OnSpawnHitFX`
  (params (HitLocation :type "Vector Structure (by ref)"))
  (`|ExecutionSequence`
    (:`then_0`
      (bind _impactsound (`self.ImpactSound`)
        (:`then`
          (`GameplayStatics.PlaySoundAtLocation` _impactsound HitLocation (struct) 1.0 1.0 0.0 null null null null))
        (:`else`)))
    (:`then_1`
      (bind _impactfx (`self.ImpactFX`)
        (:`then`
          (`NiagaraFunctionLibrary.SpawnSystemAtLocation` _impactfx HitLocation))
        (:`else`)))))

(fn `UserConstructionScript`)